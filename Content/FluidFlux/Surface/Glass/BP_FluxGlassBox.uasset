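; Glass box actor in the Fluid Flux surface system that describes itself as an SDF shape source.
; GetShapes returns a single SDF shape built from the actor's location, rotation and scale, with scale multiplied by 50 to give the shape's size.
; GetSourceType returns a fixed enum value, and the event graph and construction script add no logic of their own.
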(event EventBeginPlay
  (|CallParentFunction) ; This node is disabled and will not be called.\nDrag off pins to build functionality.
)

(fn ConstructionScript
  (|CallParentFunction))

(fn GetShapes
  (return (Utilities|Array|MakeArray (Utilities|Struct|MakeBS_SDFShape (Math|Transform|MakeTransform (Transformation|GetActorLocation) (Transformation|GetActorRotation) (* (Transformation|GetActorScale3D) 5e+01)) 0.0))))

(fn GetSourceType
  (return "NewEnumerator0"))