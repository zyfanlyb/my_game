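; Fluid Flux volume actor that rasterizes source shape actors into a signed distance field, stored as Z slices tiled in a 2D render target.
; A data asset carries texture and bounds to preview actors via surface and renderer interfaces.
; Captures run on construction, BeginPlay, source changes and optional interval Tick.
; A Niagara rasterizer takes shape arrays when available; otherwise materials draw shapes, heightmaps and per-slice splines.
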(event Custom|Capture
  (if (Variables|Capture|GetAffectWorld)
    (Utilities|Time|SetTimerbyFunctionName 0 "CaptureDistanceFields" (Variables|Capture|GetRuntimeCaptureDelay))))

(event EventBeginPlay
  (if (Variables|Capture|GetAffectWorld)
    (Initialize|InitializeAll)
    (Utilities|FlowControl|Delay 0.2)
    (Capture|CaptureDistanceFields)))

(event EventOnCapturedShapeChanged
  (params (Source :type Actor%20Object%20Reference))
  (if (Variables|Capture|GetAffectWorld)
    (if (>= (Utilities|Array|FindItem (Variables|Capture|GetSourceShapeActors) Source) 0)
      (Capture|CaptureDistanceFields))))

(event EventTick
  (params (DeltaSeconds :type Float%20%28single-precision%29))
  (Variables|Default|GetNiagaraRasterizer
    (:then
      (Capture|CapturewithNiagara))
    (:else
      (Capture|CapturewithBlueprints))))

(fn ConstructionScript
  (if (Variables|Capture|GetAffectWorld)
    (Initialize|InitializeAll)
    (CallFunction|Capture)))

(fn ApplytoActors
  (if (Variables|Capture|GetAffectWorld)
    (for _array_element (Variables|Capture|GetTargetPreviewActors)
      (LocalVariables|SetPreviewActor _array_element)
      (Utilities|FlowControl|Sequence
        (:then_0
          (if (Utilities|DoesObjectImplementInterface (LocalVariables|GetPreviewActor) "/Game/FluidFlux/Surface/Blueprints/BPI_FluxSurface.BPI_FluxSurface_C")
            (Class|BPIFluxSurface|SetSignedDistanceFieldMask(Message) (LocalVariables|GetPreviewActor) (Variables|Capture|GetVolumeDataAsset))))
        (:then_1
          (if (Utilities|DoesObjectImplementInterface (LocalVariables|GetPreviewActor) "/Game/FluidFlux/Tools/DistanceField/Blueprints/BPI_SDFRenderer.BPI_SDFRenderer_C")
            (Class|BPISDFRenderer|ApplySignedDistanceField(Message) (LocalVariables|GetPreviewActor) (Variables|Capture|GetVolumeDataAsset))))))
    (Variables|Default|GetDebug
      (:then
        (Default|ApplyMaterialParameters (Variables|Capture|GetVolumeDataAsset) (Utilities|Array|MakeArray (Variables|Default|GetDebugMaterial))))
      (:else))))

(fn CaptureDistanceFields
  (Utilities|FlowControl|Sequence
    (:then_0
      (Variables|Default|GetNiagaraRasterizer
        (:then
          (Capture|CapturewithNiagara))
        (:else
          (Capture|CapturewithBlueprints))))
    (:then_1
      (Capture|ApplytoActors))))

(fn InitializeAll
  (Utilities|FlowControl|Sequence
    (:then_0
      (Initialize|InitializeRenderTargets))
    (:then_1
      (Initialize|InitializeArea))
    (:then_2
      (Initialize|InitlializeBlueprintRasterizer))
    (:then_3
      (Initialize|InitializeNiagaraRasterizer))
    (:then_4
      (CallFunction|SetUpdateFrequency (Variables|Capture|GetUpdateFrequency)))))

(fn InitializeRenderTargets
  (bind _resolution (Variables|Capture|GetResolution))
  (Variables|Default|SetTiles (CallFunction|FramestoTiles (.z (Variables|Capture|GetResolution))))
  (bind _newtexture (CallFunction|RecreateRenderTarget (Variables|Capture|GetVolumeTexture) (* (.x (Variables|Default|GetTiles)) (.x _resolution)) (* (.y (Variables|Default|GetTiles)) (.y _resolution)) (select (Variables|Capture|GetHighPrecission) "RTF_R16f" "RTF_R8") "(R=1.000000,G=1.000000,B=1.000000,A=1.000000)" 0 false true))
  (bind _output_get (Variables|Capture|SetVolumeTexture _newtexture))
  (Variables|/Script/Engine.Texture|SetSRGB _output_get false))

(fn InitlializeBlueprintRasterizer
  (Utilities|Array|Clear (Variables|Materials|GetSDFInstances))
  (Utilities|FlowControl|Sequence
    (:then_0
      (Variables|Materials|GetSDFShapeInstance
        (:then
          _)
        (:else
          (bind _returnvalue (Rendering|Material|CreateDynamicMaterialInstance "/Game/FluidFlux/Tools/DistanceField/Materials/MI_RenderSDFShape.MI_RenderSDFShape" "None" "None" :!class /Script/Engine.KismetMaterialLibrary))
          (Variables|Materials|SetSDFShapeInstance _returnvalue)))
      (Utilities|Array|Add (Variables|Materials|GetSDFInstances) (Variables|Materials|GetSDFShapeInstance)))
    (:then_1
      (Variables|Materials|GetSDFHeightmapInstance
        (:then
          _)
        (:else
          (bind _returnvalue_2 (Rendering|Material|CreateDynamicMaterialInstance "/Game/FluidFlux/Tools/DistanceField/Materials/MI_RenderSDFHeightnap.MI_RenderSDFHeightnap" "None" "None" :!class /Script/Engine.KismetMaterialLibrary))
          (Variables|Materials|SetSDFHeightmapInstance _returnvalue_2)))
      (Utilities|Array|Add (Variables|Materials|GetSDFInstances) (Variables|Materials|GetSDFHeightmapInstance)))
    (:then_2
      (Variables|Materials|GetSDFTileInstance
        (:then
          _)
        (:else
          (bind _returnvalue_3 (Rendering|Material|CreateDynamicMaterialInstance "/Game/FluidFlux/Tools/DistanceField/Materials/M_RenderSDFTile.M_RenderSDFTile" "None" "None" :!class /Script/Engine.KismetMaterialLibrary))
          (Variables|Materials|SetSDFTileInstance _returnvalue_3)))
      (Utilities|Array|Add (Variables|Materials|GetSDFInstances) (Variables|Materials|GetSDFTileInstance)))
    (:then_3
      (Default|ApplyMaterialParameters (Variables|Capture|GetVolumeDataAsset) (Variables|Materials|GetSDFInstances))
      (Rendering|Material|SetScalarParameterValue (Variables|Materials|GetSDFInstances) "SDFInverse" (Math|Float|SelectFloat -1.0 1.0 (Variables|Capture|GetInverse)) :!class /Script/Engine.MaterialInstanceDynamic))))

(fn InitializeNiagaraRasterizer
  (Variables|Capture|GetNiagaraSystem
    (:then
      (Utilities|FlowControl|Sequence
        (:then_0
          (Variables|Default|GetNiagaraRasterizer
            (:then)
            (:else
              (bind _returnvalue (AddComponent|AddNiagaraComponent false))
              (bind _output_get (Variables|Default|SetNiagaraRasterizer _returnvalue))
              (Class|NiagaraComponent|SetAsset _output_get (Variables|Capture|GetNiagaraSystem) true))))
        (:then_1
          (Class|NiagaraComponent|SetAgeUpdateMode (Variables|Default|GetNiagaraRasterizer) "DesiredAgeNoSeek")
          (Class|NiagaraComponent|SetLockDesiredAgeDeltaTimetoSeekDelta (Variables|Default|GetNiagaraRasterizer) true))
        (:then_2
          (Default|ApplyNiagaraParameters (Variables|Capture|GetVolumeDataAsset) (Variables|Default|GetNiagaraRasterizer)))))
    (:else)))

(fn InitializeArea
  (Utilities|FlowControl|Sequence
    (:then_0
      (Variables|Capture|SetWorldTexelSize (Math|Vector|MakeVector (.x (Variables|Capture|GetWorldTexelSize)) (.x (Variables|Capture|GetWorldTexelSize)) (.z (Variables|Capture|GetWorldTexelSize))))
      (Variables|Capture|SetVolumeSize (* (Variables|Capture|GetWorldTexelSize) (Variables|Capture|GetResolution)))
      (Transformation|SetRelativeScale3D (Variables|Default|GetBounds) (Variables|Capture|GetVolumeSize))
      (Transformation|SetActorRotation "0, 0, 0"))
    (:then_1
      (Variables|Capture|GetVolumeDataAsset
        (:then)
        (:else
          (bind _returnvalue (Game|ConstructObjectfromClass self "/Game/FluidFlux/Tools/DistanceField/Blueprints/PDA_FluxSignedDistanceField.PDA_FluxSignedDistanceField_C"))
          (Variables|Capture|SetVolumeDataAsset _returnvalue))))
    (:then_2
      (Variables|Capture|GetVolumeDataAsset
        (:then
          (Default|SetData (Variables|Capture|GetVolumeDataAsset) (Variables|Capture|GetVolumeTexture) (Variables|Capture|GetVolumeSize) (Transformation|GetWorldLocation (Variables|Default|GetBounds)) (Variables|Default|GetTiles) (Math|Float|SelectFloat (* (Variables|Capture|GetDistanceRange) -1.0) (Variables|Capture|GetDistanceRange) false)))
        (:else)))
    (:then_3
      (bind _debug (Variables|Default|GetDebug)
        (:then
          (Transformation|SetRelativeScale3D _debug (* (Variables|Capture|GetVolumeSize) 0.01))
          (bind _returnvalue_2 (Rendering|Material|CreateDynamicMaterialInstance _debug 0 0 "None" :!class /Script/Engine.PrimitiveComponent))
          (Variables|Default|SetDebugMaterial _returnvalue_2))
        (:else)))))

(fn CapturewithNiagara
  (Variables|Default|GetNiagaraRasterizer
    (:then
      (Utilities|FlowControl|Sequence
        (:then_0
          (bind _array_element (Utilities|ForEachLoopFast (Variables|Capture|GetSourceShapeActors))
            (:LoopBody
              (bind _type (Class|BPISDFSource|GetSourceType(Message) _array_element))
              (if (Utilities|Enum|Equal(Enum) _type "NewEnumerator0")
                (bind _shapes (Class|BPISDFSource|GetShapes(Message) _array_element))
                (bind _array_element_2 (Utilities|ForEachLoopFast _shapes)
                  (:LoopBody
                    (Utilities|Array|Add (LocalVariables|GetShapeLocationRadius) (Math|Vector4|MakeVector4 (.X (Math|Vector|BreakVector (.location (.Transform (Utilities|Struct|BreakBS_SDFShape _array_element_2))))) (.Y (Math|Vector|BreakVector (.location (.Transform (Utilities|Struct|BreakBS_SDFShape _array_element_2))))) (.Z (Math|Vector|BreakVector (.location (.Transform (Utilities|Struct|BreakBS_SDFShape _array_element_2))))) (.Radius (Utilities|Struct|BreakBS_SDFShape _array_element_2))))
                    (Utilities|Array|Add (LocalVariables|GetShapeSize) (.scale (.Transform (Utilities|Struct|BreakBS_SDFShape _array_element_2))))
                    (Utilities|Array|Add (LocalVariables|GetShapeForward) (Math|Vector|GetForwardVector (Class|KismetMathLibrary|NegateRotator (.rotation (.Transform (Utilities|Struct|BreakBS_SDFShape _array_element_2))))))
                    (Utilities|Array|Add (LocalVariables|GetShapeUp) (Math|Vector|GetUpVector (Class|KismetMathLibrary|NegateRotator (.rotation (.Transform (Utilities|Struct|BreakBS_SDFShape _array_element_2))))))))))))
        (:then_1
          (Class|NiagaraDataInterfaceArrayFunctionLibrary|SetNiagaraArrayVector4 (Variables|Default|GetNiagaraRasterizer) "ShapeLocationRadius" (LocalVariables|GetShapeLocationRadius))
          (Class|NiagaraDataInterfaceArrayFunctionLibrary|SetNiagaraArrayVector (Variables|Default|GetNiagaraRasterizer) "ShapeSize" (LocalVariables|GetShapeSize))
          (Class|NiagaraDataInterfaceArrayFunctionLibrary|SetNiagaraArrayVector (Variables|Default|GetNiagaraRasterizer) "ShapeForward" (LocalVariables|GetShapeForward))
          (Class|NiagaraDataInterfaceArrayFunctionLibrary|SetNiagaraArrayVector (Variables|Default|GetNiagaraRasterizer) "ShapeUp" (LocalVariables|GetShapeUp)))
        (:then_2
          (Class|NiagaraComponent|AdvanceSimulation (Variables|Default|GetNiagaraRasterizer) 1 1.0))))
    (:else)))

(fn CapturewithBlueprints
  (Rendering|ClearRenderTarget2D (Variables|Capture|GetVolumeTexture))
  (for _array_element (Variables|Capture|GetSourceShapeActors)
    (LocalVariables|SetCapturedActor _array_element)
    (bind _capturedactor (LocalVariables|GetCapturedActor)
      (:then
        (bind _type (Class|BPISDFSource|GetSourceType(Message) _capturedactor))
        (switch Utilities|FlowControl|Switch|SwitchonBPE_SDFSourceType _type
          (:NewEnumerator1
            (Class|BPISDFSource|PrepareMaterial(Message) (LocalVariables|GetCapturedActor) (Variables|Materials|GetSDFHeightmapInstance))
            (Rendering|DrawMaterialtoRenderTarget (Variables|Capture|GetVolumeTexture) (Variables|Materials|GetSDFHeightmapInstance)))
          (:NewEnumerator0
            (bind _shapes (Class|BPISDFSource|GetShapes(Message) (LocalVariables|GetCapturedActor)))
            (bind _array_element_2 (Utilities|ForEachLoopFast _shapes)
              (:LoopBody
                (Rendering|Material|SetVectorParameterValue (Variables|Materials|GetSDFShapeInstance) "ShapeLocationRadius" (Math|Color|MakeColor (.X (Math|Vector|BreakVector (.location (.Transform (Utilities|Struct|BreakBS_SDFShape _array_element_2))))) (.Y (Math|Vector|BreakVector (.location (.Transform (Utilities|Struct|BreakBS_SDFShape _array_element_2))))) (.Z (Math|Vector|BreakVector (.location (.Transform (Utilities|Struct|BreakBS_SDFShape _array_element_2))))) (.Radius (Utilities|Struct|BreakBS_SDFShape _array_element_2))) :!class /Script/Engine.MaterialInstanceDynamic)
                (Rendering|Material|SetVectorParameterValue (Variables|Materials|GetSDFShapeInstance) "ShapeSize" (Math|Conversions|ToLinearColor(Vector) (.scale (.Transform (Utilities|Struct|BreakBS_SDFShape _array_element_2)))) :!class /Script/Engine.MaterialInstanceDynamic)
                (Rendering|Material|SetVectorParameterValue (Variables|Materials|GetSDFShapeInstance) "ShapeForward" (Math|Conversions|ToLinearColor(Vector) (Math|Vector|GetForwardVector (Class|KismetMathLibrary|NegateRotator (.rotation (.Transform (Utilities|Struct|BreakBS_SDFShape _array_element_2)))))) :!class /Script/Engine.MaterialInstanceDynamic)
                (Rendering|Material|SetVectorParameterValue (Variables|Materials|GetSDFShapeInstance) "ShapeUp" (Math|Conversions|ToLinearColor(Vector) (Math|Vector|GetUpVector (Class|KismetMathLibrary|NegateRotator (.rotation (.Transform (Utilities|Struct|BreakBS_SDFShape _array_element_2)))))) :!class /Script/Engine.MaterialInstanceDynamic)
                (Rendering|DrawMaterialtoRenderTarget (Variables|Capture|GetVolumeTexture) (Variables|Materials|GetSDFShapeInstance)))))
          (:NewEnumerator3
            (Class|BPISDFSource|PrepareMaterial(Message) (LocalVariables|GetCapturedActor) (Variables|Materials|GetSDFTileInstance))
            (for _index (range 0 (- (.z (Variables|Capture|GetResolution)) 1))
              (LocalVariables|SetTileIndex _index)
              (Class|BPISDFSource|Capture(Message) (LocalVariables|GetCapturedActor) (Default|GetLayerZLocation (Variables|Capture|GetVolumeDataAsset) (LocalVariables|GetTileIndex)))
              (Rendering|Material|SetScalarParameterValue (Variables|Materials|GetSDFTileInstance) "FrameIndex" (Math|Conversions|ToFloat(Integer) (LocalVariables|GetTileIndex)) :!class /Script/Engine.MaterialInstanceDynamic)
              (Rendering|DrawMaterialtoRenderTarget (Variables|Capture|GetVolumeTexture) (Variables|Materials|GetSDFTileInstance))))))
      (:else))))

(fn SetUpdateFrequency
  (params (Interval :type Float%20%28double-precision%29))
  (bind _output_get (Variables|Capture|SetUpdateFrequency Interval))
  (if (>= _output_get 0.0)
    (Actor|Tick|SetActorTickInterval (Variables|Capture|GetUpdateFrequency))
    (Actor|Tick|SetActorTickEnabled true)
    (else
      (Actor|Tick|SetActorTickEnabled false))))