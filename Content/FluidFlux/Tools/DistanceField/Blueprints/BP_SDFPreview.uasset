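; BP_SDFPreview is a preview actor that displays Fluid Flux signed distance field data on a plane.
; On construction and BeginPlay it finds a BP_SDFVolumeDomain in the level and applies that domain's volume data asset.
; The data asset writes its parameters into a dynamic material instance, created once on the plane's first material slot and cached as DebugInstance.
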(event EventApplySignedDistanceField
  (params (DataAsset :type PDA%20Flux%20Signed%20Distance%20Field%20Object%20Reference))
  (CallFunction|CreateMaterial)
  (Default|ApplyMaterialParameters DataAsset (Utilities|Array|MakeArray (Variables|Default|GetDebugInstance))))

(event EventBeginPlay
  (CallFunction|Initialize))

(fn ConstructionScript
  (CallFunction|Initialize))

(fn Initialize
  (CallFunction|CreateMaterial)
  (bind _returnvalue (Actor|GetActorOfClass "/Game/FluidFlux/Tools/DistanceField/Blueprints/BP_SDFVolumeDomain.BP_SDFVolumeDomain_C"))
  (Utilities|IsValid _returnvalue
    (:Is%20Valid
      (CallFunction|ApplySignedDistanceField (Variables|/Game/FluidFlux/Tools/DistanceField/Blueprints/BP_SDFVolumeDomain.BP_SDFVolumeDomain_C|GetVolumeDataAsset _returnvalue)))))

(fn CreateMaterial
  (Variables|Default|GetDebugInstance
    (:then)
    (:else
      (bind _returnvalue (Rendering|Material|CreateDynamicMaterialInstance (Variables|Default|GetPlane) 0 0 "None" :!class /Script/Engine.PrimitiveComponent))
      (Variables|Default|SetDebugInstance _returnvalue))))