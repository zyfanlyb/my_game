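; FluidFlux tool actor that renders selected actors into a signed distance field texture with an orthographic scene capture.
; Initialization sizes the render target and bounds from resolution and texel size, fills a PDA_FluxSignedDistanceField asset, sets up debug display, then repaints.
; Repaint toggles material parameter collection capture flags around capturing the scene.
; Capture repeats this at a given Z, and PrepareMaterial passes the field to other materials.
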(event EventBeginPlay
  (Initialize|InitializeAll))

(event EventPrepareMaterial
  (params (Material :type Material%20Instance%20Dynamic%20Object%20Reference))
  (Default|ApplyMaterialParameters (Variables|Capture|GetDistanceFieldAsset) (Utilities|Array|MakeArray Material) "Source"))

(event EventCapture
  (params (ZPosition :type Float%20%28double-precision%29))
  (bind _returnvalue (Transformation|GetActorLocation))
  (Transformation|SetActorLocation (Math|Vector|MakeVector (.x _returnvalue) (.y _returnvalue) ZPosition) false false)
  (Capture|Repaint))

(fn ConstructionScript
  (Initialize|InitializeAll))

(fn Repaint
  (Utilities|FlowControl|Sequence
    (:then_0
      (Rendering|Material|SetScalarParameterValue "/Game/FluidFlux/Surface/Materials/MPC_FluidFlux.MPC_FluidFlux" "CaptureHeightmap" 1.0 :!class /Script/Engine.KismetMaterialLibrary)
      (Rendering|Material|SetScalarParameterValue "/Game/FluidFlux/Surface/Materials/MPC_FluidFlux.MPC_FluidFlux" "CaptureDistanceField" 1.0 :!class /Script/Engine.KismetMaterialLibrary))
    (:then_1
      (bind _array_element (Utilities|ForEachLoopFast (Variables|Capture|GetCapturedActors))
        (:LoopBody
          (Utilities|IsValid _array_element
            (:Is%20Valid
              (Class|BPISDFSource|PrepareMaterial(Message) _array_element))))))
    (:then_2
      (Rendering|Material|SetScalarParameterValue "/Game/FluidFlux/Tools/DistanceField/Materials/MPC_Glass.MPC_Glass" "GenerateZ" (.z (Transformation|GetActorLocation)) :!class /Script/Engine.KismetMaterialLibrary)
      (Rendering|Material|SetScalarParameterValue "/Game/FluidFlux/Tools/DistanceField/Materials/MPC_Glass.MPC_Glass" "DistanceRange" (Variables|Capture|GetDistanceRange) :!class /Script/Engine.KismetMaterialLibrary)
      (Rendering|SceneCapture|CaptureScene (Variables|Default|GetSceneCaptureComponent2D) :!class /Script/Engine.SceneCaptureComponent2D))
    (:then_3
      (Rendering|Material|SetScalarParameterValue "/Game/FluidFlux/Surface/Materials/MPC_FluidFlux.MPC_FluidFlux" "CaptureHeightmap" 0.0 :!class /Script/Engine.KismetMaterialLibrary)
      (Rendering|Material|SetScalarParameterValue "/Game/FluidFlux/Surface/Materials/MPC_FluidFlux.MPC_FluidFlux" "CaptureDistanceField" 0.0 :!class /Script/Engine.KismetMaterialLibrary))))

(fn InitializeAll
  (Utilities|FlowControl|Sequence
    (:then_0
      (Initialize|InitializeRenderTargets))
    (:then_1
      (Initialize|InitializeSceneCapture))
    (:then_2
      (Initialize|InitializeDataAsset))
    (:then_3
      (Initialize|InitializeDebug))
    (:then_4
      (Capture|Repaint))))

(fn InitializeRenderTargets
  (bind _captureresolution (Variables|Capture|GetCaptureResolution))
  (bind _newtexture (CallFunction|RecreateRenderTarget (Variables|Capture|GetSignedDistanceField) (.x _captureresolution) (.y _captureresolution) (select (Variables|Capture|GetHighPrecission) "RTF_R16f" "RTF_R8") "(R=1.000000,G=1.000000,B=1.000000,A=1.000000)" 0 false true))
  (Variables|Capture|SetSignedDistanceField _newtexture)
  (Variables|/Script/Engine.Texture|SetSRGB _newtexture false))

(fn InitializeSceneCapture
  (bind _captureresolution (Variables|Capture|GetCaptureResolution))
  (bind _worldtexelsize (Variables|Capture|GetWorldTexelSize))
  (bind _returnvalue (Math|Conversions|ToVector2D(IntPoint) _captureresolution))
  (bind _returnvalue_2 (* _returnvalue _worldtexelsize))
  (Variables|Capture|SetAreaSize (Math|Vector|MakeVector (.x _returnvalue_2) (.y _returnvalue_2) 1.0))
  (Utilities|FlowControl|Sequence
    (:then_0
      (Variables|Default|GetBounds
        (:then
          (Transformation|SetRelativeScale3D (Variables|Default|GetBounds) (Variables|Capture|GetAreaSize)))
        (:else)))
    (:then_1
      (Transformation|SetActorRotation "0, 0, 0")
      (Variables|/Script/Engine.SceneCaptureComponent2D|SetOrthoWidth (Variables|Default|GetSceneCaptureComponent2D) (.x (Variables|Capture|GetAreaSize)))
      (Transformation|SetRelativeLocation (Variables|Default|GetSceneCaptureComponent2D) (Math|Vector|MakeVectorNetQuantize 0.0 0.0 (.z (Variables|Capture|GetAreaSize))) false false)
      (Variables|/Script/Engine.SceneCaptureComponent|SetShowOnlyActors (Variables|Default|GetSceneCaptureComponent2D) (Variables|Capture|GetCapturedActors))
      (Variables|/Script/Engine.SceneCaptureComponent2D|SetTextureTarget (Variables|Default|GetSceneCaptureComponent2D) (Variables|Capture|GetSignedDistanceField)))))

(fn InitializeDebug
  (bind _debug (Variables|Default|GetDebug)
    (:then
      (Transformation|SetRelativeScale3D _debug (* (Variables|Capture|GetAreaSize) 0.01))
      (Rendering|SetVisibility (Variables|Default|GetDebug) (Variables|Capture|GetShowDebug) false)
      (bind _returnvalue (Rendering|Material|CreateDynamicMaterialInstance (Variables|Default|GetDebug) 0 0 "None" :!class /Script/Engine.PrimitiveComponent))
      (LocalVariables|SetMaterialinstance _returnvalue)
      (Default|ApplyMaterialParameters (Variables|Capture|GetDistanceFieldAsset) (Utilities|Array|MakeArray (LocalVariables|GetMaterialinstance))))
    (:else)))

(fn InitializeDataAsset
  (Utilities|FlowControl|Sequence
    (:then_0
      (Variables|Capture|GetDistanceFieldAsset
        (:then)
        (:else
          (bind _returnvalue (Game|ConstructObjectfromClass self "/Game/FluidFlux/Tools/DistanceField/Blueprints/PDA_FluxSignedDistanceField.PDA_FluxSignedDistanceField_C"))
          (Variables|Capture|SetDistanceFieldAsset _returnvalue))))
    (:then_1
      (Variables|Capture|GetDistanceFieldAsset
        (:then
          (Default|SetData (Variables|Capture|GetDistanceFieldAsset) (Variables|Capture|GetSignedDistanceField) (Variables|Capture|GetAreaSize) (Transformation|GetWorldLocation (Variables|Default|GetBounds)) (Utilities|Struct|MakeIntPoint 1 1) (Math|Float|SelectFloat (* (Variables|Capture|GetDistanceRange) -1.0) (Variables|Capture|GetDistanceRange) (Variables|Capture|GetInverse))))
        (:else)))
    (:then_2
      (return))))

(fn GenerateDistanceFields
  (if (Utilities|DoesObjectImplementInterface self "/Game/FluidFlux/Tools/DistanceField/Blueprints/BPI_SDFSource.BPI_SDFSource_C")
    (bind _outactors (Actor|GetAllActorswithInterface "/Game/FluidFlux/Tools/DistanceField/Blueprints/BPI_SDFVolume.BPI_SDFVolume_C"))
    (Class|BPISDFVolume|OnCapturedShapeChanged(Message) _outactors self)))

(fn GetShapes
  (return 0))

(fn GetSourceType
  (return "NewEnumerator3"))