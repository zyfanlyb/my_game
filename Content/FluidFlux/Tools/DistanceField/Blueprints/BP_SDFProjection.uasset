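; Fluid Flux SDF projection actor that captures a depth map of selected actors within a box volume for distance field tools.
; The construction script sizes the box and an R16f render target, then runs an orthographic scene capture while toggling the CaptureHeightmap collection parameter.
; Plane and optional debug materials receive the depth map.
; PrepareMaterial passes capture axes, position, size, depth map and distance range to any material for projection.
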(event EventPrepareMaterial
  (params (Material :type Material%20Instance%20Dynamic%20Object%20Reference))
  (CallFunction|ApplyMaterial Material))

(fn ConstructionScript
  (bind _volume (Variables|Default|GetVolume))
  (bind _resolution (Variables|Default|GetResolution))
  (Utilities|FlowControl|Sequence
    (:then_0
      (Transformation|SetWorldScale3D (Variables|Default|GetBox) (/ (Variables|Default|GetVolume) 1e+02))
      (Transformation|SetRelativeLocation (Variables|Default|GetBox) (Math|Vector|MakeVectorNetQuantize (* (.z (Variables|Default|GetVolume)) 0.5) 0.0 0.0) false false))
    (:then_1
      (bind _newtexture (CallFunction|RecreateRenderTarget (Variables|Default|GetCurrentFrame) _resolution (Math|Float|Truncate (* (Math|Conversions|ToFloat(Integer) _resolution) (/ (.y _volume) (.x _volume)))) "RTF_R16f" "(R=1.000000,G=1.000000,B=1.000000,A=1.000000)" 0 false true))
      (Variables|Default|SetCurrentFrame _newtexture)
      (Variables|/Script/Engine.Texture|SetSRGB _newtexture false))
    (:then_2
      (bind _returnvalue (Rendering|Material|CreateDynamicMaterialInstance (Variables|Default|GetPlane) 0 0 "None" :!class /Script/Engine.PrimitiveComponent))
      (bind _output_get (Variables|Default|SetMaterialInsatnce _returnvalue))
      (Rendering|Material|SetTextureParameterValue _output_get "DepthMap" (Variables|Default|GetCurrentFrame))
      (Rendering|Material|SetScalarParameterValue _output_get "FarPlane" (.z (Variables|Default|GetVolume)) :!class /Script/Engine.MaterialInstanceDynamic))
    (:then_3
      (Variables|Default|GetDebugPlane
        (:then
          (bind _returnvalue_2 (Rendering|Material|CreateDynamicMaterialInstance (Variables|Default|GetDebugPlane) 0 0 "None" :!class /Script/Engine.PrimitiveComponent))
          (bind _output_get_2 (LocalVariables|SetDebug _returnvalue_2))
          (CallFunction|PrepareMaterial _output_get_2))
        (:else)))
    (:then_4
      (Variables|/Script/Engine.SceneCaptureComponent|SetShowOnlyActors (Variables|Default|GetSceneCaptureComponent2D) (Variables|Default|GetShow%20Only%20Actors))
      (Variables|/Script/Engine.SceneCaptureComponent2D|SetOrthoWidth (Variables|Default|GetSceneCaptureComponent2D) (.x (Variables|Default|GetVolume)))
      (Variables|/Script/Engine.SceneCaptureComponent2D|SetTextureTarget (Variables|Default|GetSceneCaptureComponent2D) (Variables|Default|GetCurrentFrame))
      (Rendering|Material|SetScalarParameterValue "/Game/FluidFlux/Surface/Materials/MPC_FluidFlux.MPC_FluidFlux" "CaptureHeightmap" 1.0 :!class /Script/Engine.KismetMaterialLibrary)
      (Rendering|SceneCapture|CaptureScene (Variables|Default|GetSceneCaptureComponent2D) :!class /Script/Engine.SceneCaptureComponent2D)
      (Rendering|Material|SetScalarParameterValue "/Game/FluidFlux/Surface/Materials/MPC_FluidFlux.MPC_FluidFlux" "CaptureHeightmap" 0.0 :!class /Script/Engine.KismetMaterialLibrary)
      (Rendering|Material|SetScalarParameterValue "/Game/FluidFlux/Surface/Materials/MPC_FluidFlux.MPC_FluidFlux" "ShowPhantoms" 1.0 :!class /Script/Engine.KismetMaterialLibrary))))

(fn ApplyMaterial
  (params (Instance :type Material%20Instance%20Dynamic%20Object%20Reference))
  (bind _scenecapturecomponent2d (Variables|Default|GetSceneCaptureComponent2D))
  (Rendering|Material|SetVectorParameterValue Instance "Front" (Math|Conversions|ToLinearColor(Vector) (Math|Vector|GetForwardVector _scenecapturecomponent2d)) :!class /Script/Engine.MaterialInstanceDynamic)
  (Rendering|Material|SetVectorParameterValue Instance "Right" (Math|Conversions|ToLinearColor(Vector) (Math|Vector|GetRightVector _scenecapturecomponent2d)) :!class /Script/Engine.MaterialInstanceDynamic)
  (Rendering|Material|SetVectorParameterValue Instance "Up" (* (Math|Conversions|ToLinearColor(Vector) (Math|Vector|GetUpVector _scenecapturecomponent2d)) -1.0) :!class /Script/Engine.MaterialInstanceDynamic)
  (Rendering|Material|SetVectorParameterValue Instance "Position" (Math|Conversions|ToLinearColor(Vector) (Transformation|GetWorldLocation _scenecapturecomponent2d)) :!class /Script/Engine.MaterialInstanceDynamic)
  (Rendering|Material|SetVectorParameterValue Instance "Size" (Math|Conversions|ToLinearColor(Vector) (Variables|Default|GetVolume)) :!class /Script/Engine.MaterialInstanceDynamic)
  (Rendering|Material|SetTextureParameterValue Instance "DepthMap" (Variables|Default|GetCurrentFrame))
  (Rendering|Material|SetScalarParameterValue Instance "DistanceRange" (Variables|Default|GetDistanceRange) :!class /Script/Engine.MaterialInstanceDynamic))

(fn GetShapes
  (return 0))

(fn GetSourceType
  (return "NewEnumerator1"))